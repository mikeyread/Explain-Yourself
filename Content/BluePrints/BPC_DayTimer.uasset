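; BPC_DayTimer is a component that runs a timed day, moving the sun across the sky and signalling when the day ends.
; StartDayTimer finds the DirectionalLight tagged SkyLight and starts a day-length timer plus a near-per-frame looping timer used in place of Tick.
; DayTick accumulates delta time to lerp the sun's rotation.
; TriggerDayEnd clears both timers and calls DayEnded.
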(event Custom|TriggerDayEnd
  (Utilities|Time|ClearandInvalidateTimerbyHandle (Variables|Default|GetTickTimer))
  (Utilities|Time|ClearandInvalidateTimerbyHandle (Variables|Default|GetDayTimer))
  (Default|CallDayEnded))

(event Custom|DayTick
  (bind _output_get (Variables|Default|SetDayProgress%28Seconds%29 (+ (Variables|Default|GetDayProgress%28Seconds%29) (Utilities|Time|GetWorldDeltaSeconds))))
  (Transformation|SetActorRotation (Variables|Default|GetSun) (Math|Rotator|Lerp(Rotator) "-90.000000,-90.000000,0.000000" "0.000000,-90.000000,0.000000" (/ _output_get (* (Variables|Default|GetDayLength%28Minutes%29) 6e+01)))))

(event Custom|StartDayTimer
  (bind _outactors (Actor|GetAllActorsOfClasswithTag "/Script/Engine.DirectionalLight" "SkyLight"))
  (Variables|Default|SetSun (Utilities|Array|Get(acopy) _outactors))
  (bind _returnvalue (Utilities|Time|SetTimerbyEvent (EventDispatchers|CreateEvent :!event Custom|TriggerDayEnd) (* (Variables|Default|GetDayLength%28Minutes%29) 6e+01)))
  (Variables|Default|SetDayTimer _returnvalue)
  (bind _returnvalue_2 (Utilities|Time|SetTimerbyEvent (EventDispatchers|CreateEvent :!event Custom|DayTick) 0.001 true true))
  (Variables|Default|SetTickTimer _returnvalue_2))