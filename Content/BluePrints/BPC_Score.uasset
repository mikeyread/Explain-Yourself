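; Actor component that makes its owner scoreable in photos by holding a score value and judging whether the owner is in shot.
; On BeginPlay it adds the "Scoreable" tag to the owner.
; IsInPhoto checks that the owner lies roughly ahead using the player controller's forward vector, then confirms line of sight with a Visibility trace from the given location.
; The trace leaves persistent debug lines.
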(event EventBeginPlay
  (Utilities|Array|Add (Variables|/Script/Engine.Actor|GetTags (Components|GetOwner)) "Scoreable"))

(event EventTick
  (params (DeltaSeconds :type Float%20%28single-precision%29)))

(fn GetScore
  (return (Variables|Default|GetScore)))

(fn IsinPhoto
  (params (Player%20Location :type Vector))
  (bind _returnvalue (Components|GetOwner))
  (bind _returnvalue_2 (Transformation|GetActorLocation _returnvalue))
  (if (> (Math|Vector|DotProduct (Math|Vector|Normalize (Transformation|GetActorForwardVector (Game|GetPlayerController 0))) (Math|Vector|Normalize (- _returnvalue_2 Player%20Location))) 0.2)
    (bind _outhit (Collision|LineTraceByChannel Player%20Location _returnvalue_2 "TraceTypeQuery1" false (Utilities|Array|MakeArray (Game|Player|GetPlayerPawn 0)) "Persistent" false))
    (return (== (.hitactor _outhit) (Components|GetOwner)))))