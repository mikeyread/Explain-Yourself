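; Base interactable actor that shows an on-screen widget while the player is within range.
; When the player pawn enters the Box component, it creates an AnimationSampleUI widget, adds it to the viewport and sets the Interactable flag.
; Leaving the box removes the widget and clears the flag.
; The Interact event is an empty stub, so this Blueprint defines no interaction behavior itself.
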(event OnComponentBeginOverlap(Box)
  (params (OverlappedComponent :type Primitive%20Component%20Object%20Reference) (OtherActor :type Actor%20Object%20Reference) (OtherComp :type Primitive%20Component%20Object%20Reference) (OtherBodyIndex :type Integer) (bFromSweep :type Boolean) (SweepResult :type Hit%20Result%20Structure%20%28by%20ref%29))
  (if (== OtherActor (Game|Player|GetPlayerPawn 0))
    (bind _returnvalue (UserInterface|CreateWidget "/DatasmithContent/Blueprints/FBXImporter/UI/AnimationSampleUI.AnimationSampleUI_C"))
    (Variables|Default|SetWidget _returnvalue)
    (UserInterface|Viewport|AddtoViewport _returnvalue 0)
    (Variables|Default|SetInteractable true)))

(event OnComponentEndOverlap(Box)
  (params (OverlappedComponent :type Primitive%20Component%20Object%20Reference) (OtherActor :type Actor%20Object%20Reference) (OtherComp :type Primitive%20Component%20Object%20Reference) (OtherBodyIndex :type Integer))
  (if (== OtherActor (Game|Player|GetPlayerPawn 0))
    (Widget|RemovefromParent (Variables|Default|GetWidget))
    (Variables|Default|SetInteractable false)))

(event Custom|Interact)

(event Custom|Interacable
  (bind _returnvalue (UserInterface|CreateWidget "/DatasmithContent/Blueprints/FBXImporter/UI/AnimationSampleUI.AnimationSampleUI_C"))
  (Variables|Default|SetWidget _returnvalue)
  (UserInterface|Viewport|AddtoViewport _returnvalue 0)
  (Variables|Default|SetInteractable true))

(event Custom|NotIteractable
  (Widget|RemovefromParent (Variables|Default|GetWidget))
  (Variables|Default|SetInteractable false))

(event EventBeginPlay)

(event Collision|EventActorBeginOverlap
  (params (OtherActor :type Actor%20Object%20Reference)))

(event EventTick
  (params (DeltaSeconds :type Float%20%28single-precision%29)))

(fn ConstructionScript)