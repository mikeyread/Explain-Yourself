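; Interactable firework that damages the homework actor when used while a BP_Homework is inside its box.
; Box overlaps set a nearby flag that gates the interaction.
; Firing marks the child BP_FireWork launched, clears its score-used flag and applies its damage at random coordinates to the homework found by class lookup.
; After a delay, it deals a second, fixed-amount hit and activates the child's Niagara effect.
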(event OnComponentBeginOverlap(Box)
  (params (OverlappedComponent :type Primitive%20Component%20Object%20Reference) (OtherActor :type Actor%20Object%20Reference) (OtherComp :type Primitive%20Component%20Object%20Reference) (OtherBodyIndex :type Integer) (bFromSweep :type Boolean) (SweepResult :type Hit%20Result%20Structure%20%28by%20ref%29))
  (if (== (Utilities|GetClass OtherActor) "/Game/BluePrints/BP_Homework.BP_Homework_C")
    (Variables|Default|Sethomework%20nearby true)))

(event OnComponentEndOverlap(Box)
  (params (OverlappedComponent :type Primitive%20Component%20Object%20Reference) (OtherActor :type Actor%20Object%20Reference) (OtherComp :type Primitive%20Component%20Object%20Reference) (OtherBodyIndex :type Integer))
  (if (== (Utilities|GetClass OtherActor) "/Game/BluePrints/BP_Homework.BP_Homework_C")
    (Variables|Default|Sethomework%20nearby false)))

(event Custom|CustomEvent
  (bind _returnvalue (Math|Random|RandomFloat))
  (bind _returnvalue_2 (Math|Random|RandomFloat))
  (bind _asbp_fire_work (Utilities|Casting|CastToBP_FireWork (Variables|/Script/Engine.ChildActorComponent|GetChildActor (Variables|Default|GetChildActor))))
  (Variables|/Game/BluePrints/Scoreable/BP_FireWork.BP_FireWork_C|Setrocketloauched _asbp_fire_work true)
  (bind _returnvalue_3 (Actor|GetActorOfClass "/Game/BluePrints/BP_Homework.BP_Homework_C"))
  (Variables|/Game/BluePrints/BPC_Score.BPC_Score_C|SetScoreUsed (Variables|/Game/BluePrints/Scoreable/BP_Base_Scoreable.BP_Base_Scoreable_C|GetBPC_Score _asbp_fire_work) false)
  (Default|AddHomeworkDamage _returnvalue_3 (Math|Vector2D|MakeVector2D _returnvalue_2 _returnvalue) (Variables|/Game/BluePrints/Scoreable/BP_Base_Scoreable.BP_Base_Scoreable_C|GetDamage%20Amount _asbp_fire_work) (Variables|/Game/BluePrints/Scoreable/BP_Base_Scoreable.BP_Base_Scoreable_C|GetDamage%20Type _asbp_fire_work) (Variables|/Game/BluePrints/Scoreable/BP_Base_Scoreable.BP_Base_Scoreable_C|GetDamage%20Speed%20%280-1%29 _asbp_fire_work))
  (Utilities|FlowControl|Delay 5.0)
  (Default|AddHomeworkDamage _returnvalue_3 (Math|Vector2D|MakeVector2D _returnvalue_2 _returnvalue) 1e+01 (Variables|/Game/BluePrints/Scoreable/BP_Base_Scoreable.BP_Base_Scoreable_C|GetDamage%20Type _asbp_fire_work) (Variables|/Game/BluePrints/Scoreable/BP_Base_Scoreable.BP_Base_Scoreable_C|GetDamage%20Speed%20%280-1%29 _asbp_fire_work))
  (Components|Activation|SetActive (Variables|/Game/BluePrints/Scoreable/BP_FireWork.BP_FireWork_C|GetNiagara _asbp_fire_work) true true))

(event EventBeginPlay
  (|CallParentFunction) ; This node is disabled and will not be called.\nDrag off pins to build functionality.
)

(event Collision|EventActorBeginOverlap
  (params (OtherActor :type Actor%20Object%20Reference))
  (|CallParentFunction OtherActor) ; This node is disabled and will not be called.\nDrag off pins to build functionality.
)

(event EventTick
  (params (DeltaSeconds :type Float%20%28single-precision%29))
  (|CallParentFunction DeltaSeconds) ; This node is disabled and will not be called.\nDrag off pins to build functionality.
)

(fn ConstructionScript
  (|CallParentFunction))

(fn InteractwithObject
  (|CallParentFunction)
  (if (Variables|Default|Gethomework%20nearby)
    (CallFunction|CustomEvent)))