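; BP_SinkTap is an interactable tap that switches the kitchen sink's Niagara effect on and off.
; Its InteractWithObject override runs the parent logic, casts its owner to BP_kichyensink and toggles that actor's Niagara component.
; If the cast fails it prints a display name as debug output.
; A SetActive node is left unconnected, and the event graph holds only disabled default events.
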(event EventBeginPlay
  (|CallParentFunction) ; This node is disabled and will not be called.\nDrag off pins to build functionality.
)

(event Collision|EventActorBeginOverlap
  (params (OtherActor :type Actor%20Object%20Reference))
  (|CallParentFunction OtherActor) ; This node is disabled and will not be called.\nDrag off pins to build functionality.
)

(event EventTick
  (params (DeltaSeconds :type Float%20%28single-precision%29))
  (|CallParentFunction DeltaSeconds) ; This node is disabled and will not be called.\nDrag off pins to build functionality.
)

(fn ConstructionScript
  (|CallParentFunction))

(fn InteractwithObject
  (|CallParentFunction)
  (bind _asbp_kichyensink (Utilities|Casting|CastToBP_kichyensink (Components|GetOwner))
    (:then
      (Components|Activation|ToggleActive (Variables|/Game/BluePrints/Scoreable/BP_kichyensink.BP_kichyensink_C|GetNiagara _asbp_kichyensink)))
    (:CastFailed
      (Development|PrintString (Utilities|GetDisplayName 0)))))