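; BP_Homework is the homework object that takes damage and, once destroyed, ends the day.
; AddHomeworkDamage forwards hits to BPCHomeworkDamage, which shares the NSHomework Niagara system, always passing one fixed damage type.
; One damage type, or accumulated damage reaching a threshold, sets the Niagara destroyed flag, calls DayEnded on the game mode and releases the player's physics handle.
; A DoOnce ignores new hits for a delay of amount divided by speed.
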(event Custom|AddHomeworkDamage
  (params (DamageXY :type Vector%202D%20Structure) (DamageAmount :type Float%20%28double-precision%29) (DamageType :type E_DamageType%20Enum :default "NewEnumerator0") (Damage%20Speed%20%280-1%29 :type Float%20%28double-precision%29))
  (Utilities|FlowControl|DoOnce false :!label _label
    (:Completed
      (Utilities|FlowControl|Sequence
        (:then_0
          (if (== DamageType 3)
            (Class|NiagaraComponent|SetVariableBool (Variables|Default|GetNS_Homework) "IsDestroyed" true :!label _label_2)
            (bind _asbp_first_person_game_mode (Utilities|Casting|CastToBP_FirstPersonGameMode (Game|GetGameMode)))
            (Default|DayEnded _asbp_first_person_game_mode)
            (bind _asbp_first_person_character (Utilities|Casting|CastToBP_FirstPersonCharacter (Game|GetPlayerCharacter 0)))
            (Physics|Components|PhysicsHandle|ReleaseComponent (Variables|/Game/FirstPerson/Blueprints/BP_FirstPersonCharacter.BP_FirstPersonCharacter_C|GetPhysicsHandle _asbp_first_person_character))
            (else
              (Default|SetDamageSpeed (Variables|Default|GetBPC_HomeworkDamage) Damage%20Speed%20%280-1%29)
              (Default|AddDamage (Variables|Default|GetBPC_HomeworkDamage) DamageXY DamageAmount "NewEnumerator0")
              (bind _output_get (Variables|Default|SetTotalDamageAmount (+ DamageAmount (Variables|Default|GetTotalDamageAmount))))
              (if (>= _output_get 2.0)
                (goto _label_2)))))
        (:then_1
          (bind _output_get_2 (Variables|Default|SetCurrent%20Damage%20Amount DamageAmount))
          (bind _output_get_3 (Variables|Default|SetCurrent%20Damage%20Speed Damage%20Speed%20%280-1%29))
          (Utilities|FlowControl|Delay (/ _output_get_2 _output_get_3))
          (goto _label Reset))))))

(event EventBeginPlay
  (Variables|/Game/BluePrints/BPC_HomeworkDamage.BPC_HomeworkDamage_C|SetNS_Homework (Variables|Default|GetBPC_HomeworkDamage) (Variables|Default|GetNS_Homework)))

(fn ConstructionScript)