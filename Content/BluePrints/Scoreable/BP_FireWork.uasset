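; BP_FireWork is a scoreable firework actor that flies upward as a rocket and carries the level's BP_Homework actor with it.
; On BeginPlay it caches the BP_Homework actor it finds.
; While the Rocketloauched flag is true, each Tick raises it by a fixed, frame-rate-dependent step and teleports the homework to Sphere1's location and rotation.
; The flag is not set within this Blueprint.
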(event EventBeginPlay
  (|CallParentFunction)
  (bind _returnvalue (Actor|GetActorOfClass "/Game/BluePrints/BP_Homework.BP_Homework_C"))
  (Variables|Default|SetHomework _returnvalue))

(event Collision|EventActorBeginOverlap
  (params (OtherActor :type Actor%20Object%20Reference))
  (|CallParentFunction OtherActor) ; This node is disabled and will not be called.\nDrag off pins to build functionality.
)

(event EventTick
  (params (DeltaSeconds :type Float%20%28single-precision%29))
  (bind _sphere1 (Variables|Default|GetSphere1))
  (|CallParentFunction DeltaSeconds)
  (if (Variables|Default|Getrocketloauched)
    (Transformation|SetActorLocationAndRotation (+ (Transformation|GetActorLocation) "0.000000,0.000000,20.000000") "0, 0, 0" true true)
    (Transformation|SetActorLocationAndRotation (Variables|Default|GetHomework) (Transformation|GetWorldLocation _sphere1) (Transformation|GetWorldRotation _sphere1) true true)))

(fn ConstructionScript
  (|CallParentFunction))