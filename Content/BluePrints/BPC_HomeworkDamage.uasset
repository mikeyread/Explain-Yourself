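; BPC_HomeworkDamage is a Blueprint component that passes damage data to the NSHomework Niagara system.
; AddDamage clamps the DamageXY variable to 0–1, packs it with amount and type into a Vector4, appends that to an array and pushes the array to Niagara's DamageArray.
; SetDamageSpeed sets the system's damage speed parameter.
; Nothing here clears the array, and BeginPlay and Tick are unused.
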(event EventBeginPlay)

(event EventTick
  (params (DeltaSeconds :type Float%20%28single-precision%29)))

(fn AddDamage
  (params (DamageXY :type Vector%202D%20Structure) (DamageAmount :type Float%20%28double-precision%29) (DamageType :type E_DamageType%20Enum :default "NewEnumerator0"))
  (Utilities|Array|Add (Variables|Default|GetArray%20Data) (Math|Vector4|MakeVector4 (Math|Float|Clamp(Float) (.x DamageXY)) (Math|Float|Clamp(Float) (.y DamageXY)) DamageAmount (Math|Conversions|ToFloat(Byte) DamageType)))
  (Class|NiagaraDataInterfaceArrayFunctionLibrary|SetNiagaraArrayVector4 (Variables|Default|GetNS_Homework) "DamageArray" (Variables|Default|GetArray%20Data)))

(fn SetDamageSpeed
  (params (Damage%20Speed%20%280-1%29 :type Float%20%28double-precision%29))
  (Niagara|SetNiagaraVariable(Float) (Variables|Default|GetNS_Homework) "DamageSpeed (0-1)" Damage%20Speed%20%280-1%29))